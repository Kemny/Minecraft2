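; Player controller for a Minecraft-style game that handles hotbar tool selection and mining or block placement input.
; BeginPlay creates the player UI widget, and number keys toggle either the pickaxe or one of several block types, updating the current state, selected block and highlighted icon.
; Left mouse input fires event dispatchers based on that state: start and stop mining for the pickaxe, or a placement request for blocks.
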(event `self.ReceiveBeginPlay`
  (bind _returnvalue (`|CreateWidget` "/Game/Widgets/WBP_PlayerUI.WBP_PlayerUI_C"))
  (bind _output_get (set `self.PlayerUI` _returnvalue))
  (`UserWidget.AddToPlayerScreen` _output_get 0))

(event `Key|LeftMouseButton`
  (params (Key :type "Key Structure"))
  (:`Pressed`
    (switch `EPlayerState` (`self.CurrentState`)
      (:`Pickaxe`
        (`self.OnStartMining`))
      (:`PlaceBlock`
        (`self.OnPlaceBlockRequest`))))
  (:`Released`
    (switch `EPlayerState` (`self.CurrentState`)
      (:`Pickaxe`
        (`self.OnStopMining`)))))

(event `Key|One`
  (params (Key :type "Key Structure"))
  (:`Pressed`
    (`self.TogglePickaxe`)))

(event `Key|Two`
  (params (Key :type "Key Structure"))
  (:`Pressed`
    (`self.ToggleBlock` 2 "Dirt")))

(event `Key|Three`
  (params (Key :type "Key Structure"))
  (:`Pressed`
    (`self.ToggleBlock` 3 "Grass")))

(event `Key|Four`
  (params (Key :type "Key Structure"))
  (:`Pressed`
    (`self.ToggleBlock` 4 "Stone")))

(event `Key|Five`
  (params (Key :type "Key Structure"))
  (:`Pressed`
    (`self.ToggleBlock` 5 "Snow")))

(fn `UserConstructionScript`)