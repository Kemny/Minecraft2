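; Game mode that spawns the block terrain and places the player's pawn on it once generation finishes.
; On BeginPlay it spawns BP_TerrainManager, binds to its OnNewTerrainGenerated event and calls CreateTerrain.
; When that event fires, it runs an object-type line trace from just above the terrain's center, derived from block size and count, with no end point set.
; Player 0's pawn moves to the trace's hit location, without checking for a hit.
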(event `self.ReceiveBeginPlay`
  (bind _returnvalue (`|SpawnActorFromClass` "/Game/Blueprints/BP_TerrainManager.BP_TerrainManager_C" (`KismetMathLibrary.MakeTransform` (0.0 0.0 0.0)) "Undefined" "OverrideRootScale" null null))
  (bind _output_get (set `self.TerrainManager` _returnvalue))
  (add `TerrainManager.OnNewTerrainGenerated` _output_get (delegate `On Terrain Generated`))
  (`TerrainManager.CreateTerrain` _output_get))

(event `On Terrain Generated`
  (bind _terrainmanager (`self.TerrainManager`))
  (bind _blocksize (`TerrainManager.BlockSize` _terrainmanager))
  (bind (_blockcount_x _blockcount_y _blockcount_z) (break `VectorByte` (`TerrainManager.BlockCount` _terrainmanager)))
  (bind _returnvalue (/ _blocksize 2))
  (bind _outhit (`KismetSystemLibrary.LineTraceSingleForObjects` (`KismetMathLibrary.MakeVector` (`KismetMathLibrary.Conv_IntToDouble` (* _returnvalue (`KismetMathLibrary.Conv_ByteToInt` _blockcount_x))) (`KismetMathLibrary.Conv_IntToDouble` (* _returnvalue (`KismetMathLibrary.Conv_ByteToInt` _blockcount_y))) (`KismetMathLibrary.Conv_IntToDouble` (+ (* _blocksize (`KismetMathLibrary.Conv_ByteToInt` _blockcount_z)) 100))) (0.0 0.0 0.0) (`|MakeArray` "ObjectTypeQuery7" :!type "EObjectTypeQuery Enum") true))
  (`self.K2_SetActorLocation` (`Controller.K2_GetPawn` (`GameplayStatics.GetPlayerController` 0)) (`.Location` (`GameplayStatics.BreakHitResult` _outhit)) false false))

(fn `UserConstructionScript`)